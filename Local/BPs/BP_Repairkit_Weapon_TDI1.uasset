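; Inventory item Blueprint for a weapon repair kit that is used up on a target item.
; HandleDurabilityLoss stores the item and controller, then on the server deletes one kit from the owner's inventory.
; A successful deletion passes both to OnConsumedFromInventory; no durability math appears in this graph.
; CanBeDroppedOnItem calls its parent but ignores the result, accepting any target.
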(event EventHandleDurabilityLoss
  (params (Item :type Game%20Item%20Object%20Reference) (Controller :type Conan%20Player%20Controller%20Object%20Reference))
  (bind _returnvalue (Class|GameItem|GetOwnerInventory))
  (bind _output_get (Variables|Default|SetLocatItem Item))
  (Utilities|IsValid _output_get
    (:Is%20Valid
      (Variables|Default|SetLocalControler Controller)
      (if (Networking|IsServer)
        ;[1 1 1] Consume Repair Kit from inventory
        (Utilities|IsValid _returnvalue
          (:Is%20Valid
            (bind _returnvalue_2 (Class|ItemInventory|DeleteItems _returnvalue (Class|ItemInventory|GetItemIndex _returnvalue self) "consumed" 1))
            (if _returnvalue_2
              (CallFunction|OnConsumedfromInventory (Variables|Default|GetLocalControler) (Variables|Default|GetLocatItem)))))))))

(fn CanbeDroppedonItem
  (params (TargetItem :type Game%20Item%20Object%20Reference))
  (|CallParentFunction TargetItem)
  (return true))